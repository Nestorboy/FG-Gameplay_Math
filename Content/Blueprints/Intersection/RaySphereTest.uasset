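; RaySphereTest is a debug test that checks a ray against a sphere at the bottom cap of the player's capsule.
; Each tick it casts the ray from its own location along its forward vector and calls SphereRay using the capsule's radius.
; A hit draws a green line and point at the contact; a miss draws a fixed-length red line.
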(event EventBeginPlay)

(event EventTick
  (params (DeltaSeconds :type Float%20%28single-precision%29))
  (bind _returnvalue (Math|Vector|GetForwardVector))
  (bind _returnvalue_2 (Transformation|GetWorldLocation))
  (bind _returnvalue_3 (Game|GetPlayerCharacter 0))
  (bind _capsulecomponent (Variables|/Script/Engine.Character|GetCapsuleComponent _returnvalue_3))
  (bind (_contactpoint _returnvalue_4) (Class|IntersectionLibrary|SphereRay (+ (Transformation|GetWorldLocation _capsulecomponent) (* (* (Math|Vector|GetUpVector _capsulecomponent) (Class|CapsuleComponent|GetScaledCapsuleHalfHeightWithoutHemisphere _capsulecomponent)) -1.0)) (Variables|/Script/Engine.CapsuleComponent|GetCapsuleRadius _capsulecomponent) _returnvalue_2 _returnvalue))
  (Rendering|Debug|DrawDebugLine _returnvalue_2 (select _returnvalue_4 _contactpoint (+ _returnvalue_2 (* _returnvalue 1e+03))) (select _returnvalue_4 "(R=0.000000,G=1.000000,B=0.000000,A=1.000000)" "(R=1.000000,G=0.000000,B=0.000000,A=1.000000)") 0.0 0.0)
  (if _returnvalue_4
    (Rendering|Debug|DrawDebugPoint _contactpoint 2e+01 "(R=0.000000,G=1.000000,B=0.000000,A=1.000000)" 0.0)))