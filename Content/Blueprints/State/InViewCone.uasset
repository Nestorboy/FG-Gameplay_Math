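; InViewCone is a debug test that shows whether the player character falls within a view cone projected along its forward vector.
; Each Tick feeds a point low on the player's capsule, at the bottom hemisphere's center, into a PointSphericalSector check with fixed radius and angle.
; It draws a debug line from its own location to that point, green when inside the sector and red when outside.
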(event EventBeginPlay)

(event EventTick
  (params (DeltaSeconds :type Float%20%28single-precision%29))
  (bind _returnvalue (Transformation|GetWorldLocation))
  (bind _returnvalue_2 (Game|GetPlayerCharacter 0))
  (bind _capsulecomponent (Variables|/Script/Engine.Character|GetCapsuleComponent _returnvalue_2))
  (bind _returnvalue_3 (Transformation|GetWorldLocation _capsulecomponent))
  (bind _returnvalue_4 (Math|Vector|GetUpVector _capsulecomponent))
  (bind _returnvalue_5 (Class|CapsuleComponent|GetScaledCapsuleHalfHeightWithoutHemisphere _capsulecomponent))
  (bind _returnvalue_6 (* _returnvalue_4 _returnvalue_5))
  (bind _returnvalue_7 (* _returnvalue_6 -1.0))
  (bind _returnvalue_8 (+ _returnvalue_3 _returnvalue_7))
  (bind _returnvalue_9 (Class|OverlapLibrary|PointSphericalSector _returnvalue_8 _returnvalue (Math|Vector|GetForwardVector) 5e+02 65.0))
  (Rendering|Debug|DrawDebugLine _returnvalue _returnvalue_8 (select _returnvalue_9 "(R=0.000000,G=1.000000,B=0.000000,A=1.000000)" "(R=1.000000,G=0.000000,B=0.000000,A=1.000000)") 0.0 0.0))