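; BP_Ball is a ball actor with hand-written physics that the player can push around.
; Each tick it applies gravity to a stored Velocity, offsets itself by it, then damps horizontal motion.
; It tests its sphere against the player capsule's bottom hemisphere and a horizontal floor plane, drawing debug contact points.
; On contact, the depenetration vector both corrects position and is added to Velocity, producing the push or bounce.
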(event Custom|ResolvePlayerCollision
  (bind (_contactpoint _returnvalue) (Class|IntersectionLibrary|SphereSphere (Transformation|GetActorLocation) (Variables|Default|GetRadius) (Variables|Default|GetPlayerBottomHemisphere) (Variables|/Script/Engine.CapsuleComponent|GetCapsuleRadius (Variables|/Script/Engine.Character|GetCapsuleComponent (Game|GetPlayerCharacter 0)))))
  (if _returnvalue
    (Rendering|Debug|DrawDebugPoint _contactpoint 1e+01 "(R=0.000000,G=1.000000,B=0.000000,A=1.000000)" 1.0)
    (CallFunction|AddForce (CallFunction|ComputeDepenetration _contactpoint))
    (Transformation|AddActorWorldOffset (CallFunction|ComputeDepenetration _contactpoint))))

(event Custom|ResolveFloorCollision
  (bind (_contactpoint _returnvalue) (Class|IntersectionLibrary|SpherePlane (Transformation|GetActorLocation) (Variables|Default|GetRadius) (Math|Vector|MakeVector 0.0 0.0 0.0) (Math|Vector|MakeVector 0.0 0.0 1.0)))
  (if _returnvalue
    (Rendering|Debug|DrawDebugPoint _contactpoint 1e+01 "(R=0.000000,G=1.000000,B=0.000000,A=1.000000)" 1.0)
    (CallFunction|AddForce (CallFunction|ComputeDepenetration _contactpoint))
    (Transformation|AddActorWorldOffset (CallFunction|ComputeDepenetration _contactpoint))))

(event Custom|ApplyGravity
  (params (DeltaTime :type Float%20%28double-precision%29))
  (CallFunction|AddForce (Math|Vector|MakeVector 0.0 0.0 (* DeltaTime -9.81)))
  (Transformation|AddActorWorldOffset (Variables|Default|GetVelocity)))

(event Custom|ApplyFriction
  (params (DeltaTime :type Float%20%28double-precision%29))
  (bind _velocity (Variables|Default|GetVelocity))
  (CallFunction|AddForce (* (- (Class|KismetMathLibrary|VectorProjectontoNormal _velocity "0.000000,0.000000,1.000000") _velocity) (* DeltaTime 2.0))))

(event EventBeginPlay)

(event EventTick
  (params (DeltaSeconds :type Float%20%28single-precision%29))
  (Variables|Default|SetPlayerBottomHemisphere (CallFunction|GetPlayerBottomHemisphere))
  (CallFunction|ApplyGravity DeltaSeconds)
  (CallFunction|ApplyFriction DeltaSeconds)
  (CallFunction|ResolvePlayerCollision)
  (CallFunction|ResolveFloorCollision))

(fn ConstructionScript)

(fn GetPlayerBottomHemisphere
  (bind _returnvalue (Game|GetPlayerCharacter 0))
  (bind _capsulecomponent (Variables|/Script/Engine.Character|GetCapsuleComponent _returnvalue))
  (return (+ (Transformation|GetWorldLocation _capsulecomponent) (* (* (Math|Vector|GetUpVector _capsulecomponent) (Class|CapsuleComponent|GetScaledCapsuleHalfHeightWithoutHemisphere _capsulecomponent)) -1.0))))

(fn ComputeDepenetration
  (params (Point :type Vector))
  (return (- Point (+ (* (Math|Vector|Normalize (- Point (Transformation|GetActorLocation))) (Variables|Default|GetRadius)) (Transformation|GetActorLocation)))))

(fn AddForce
  (params (Force :type Vector))
  (Variables|Default|SetVelocity (+ Force (Variables|Default|GetVelocity))))

(fn FlattenVelocity
  (params (Normal :type Vector))
  (Variables|Default|SetVelocity (Math|Vector|ProjectVectorontoPlane (Variables|Default|GetVelocity) Normal)))